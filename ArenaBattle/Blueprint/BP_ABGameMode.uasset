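; BP_ABGameMode is the game mode that ends a round and shows whether the player cleared or failed the game.
; GameCleared and GameFailed set the IsGameCleared flag, then both call ShowResult.
; ShowResult freezes player 0's character by setting its movement mode to None, then creates the WBP_GameResult widget, adds it to the viewport and passes it the outcome.
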(event `GameFailed`
  (set `self.IsGameCleared` false)
  (`self.ShowResult`))

(event `GameCleared`
  (set `self.IsGameCleared` true)
  (`self.ShowResult`))

(event `ShowResult`
  (`|ExecutionSequence`
    (:`then_0`
      (bind `_as캐릭터` (cast `Character` (`Controller.K2_GetPawn` (`GameplayStatics.GetPlayerController` 0))))
      (`CharacterMovementComponent.SetMovementMode` (`Character.CharacterMovement` `_as캐릭터`) "MOVE_None" 0))
    (:`then_1`
      (bind _returnvalue (`|CreateWidget` "/Game/ArenaBattle/UI/WBP_GameResult.WBP_GameResult_C" (`GameplayStatics.GetPlayerController` 0)))
      (`UserWidget.AddToViewport` _returnvalue 0)
      (`/Game/ArenaBattle/UI/WBP_GameResult.SetResult` _returnvalue (`self.IsGameCleared`)))))

(fn `UserConstructionScript`)